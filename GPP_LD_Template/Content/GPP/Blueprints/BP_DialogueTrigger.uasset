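; BP_DialogueTrigger is a trigger volume that plays a one-time dialogue when the player walks into it.
; On box overlap by BP_PlayerCharacter, it disables the character's movement and spawns a WB_Dialogue widget.
; It passes the widget the player reference and the trigger's DialogueText, starts the typing effect, then sets HasPlayed so it does not fire again.
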(event OnComponentBeginOverlap(Box)
  (params (OverlappedComponent :type Primitive%20Component%20Object%20Reference) (OtherActor :type Actor%20Object%20Reference) (OtherComp :type Primitive%20Component%20Object%20Reference) (OtherBodyIndex :type Integer) (bFromSweep :type Boolean) (SweepResult :type Hit%20Result%20Structure%20%28by%20ref%29))
  (bind _asbp_player_character (Utilities|Casting|CastToBP_PlayerCharacter OtherActor))
  (if (not (Variables|Default|GetHasPlayed))
    (Pawn|Components|CharacterMovement|DisableMovement (Variables|/Script/Engine.Character|GetCharacterMovement _asbp_player_character))
    (bind _returnvalue (UserInterface|CreateWidget "/Game/GPP/Blueprints/WB_Dialogue.WB_Dialogue_C"))
    (Variables|/Game/GPP/Blueprints/WB_Dialogue.WB_Dialogue_C|SetPlayerRef _returnvalue _asbp_player_character)
    (UserInterface|Viewport|AddtoViewport _returnvalue 0)
    (Variables|/Game/GPP/Blueprints/WB_Dialogue.WB_Dialogue_C|SetFullText _returnvalue (Variables|Default|GetDialogueText))
    (Default|StartType _returnvalue)
    (Variables|Default|SetHasPlayed true)))

(event EventBeginPlay)

(event Collision|EventActorBeginOverlap
  (params (OtherActor :type Actor%20Object%20Reference)))

(event EventTick
  (params (DeltaSeconds :type Float%20%28single-precision%29)))

(fn ConstructionScript)