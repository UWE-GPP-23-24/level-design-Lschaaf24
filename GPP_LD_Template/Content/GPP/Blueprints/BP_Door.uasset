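; Door actor that opens by moving vertically once KeyCollected has been called as many times as KeysRequired.
; If a Camera is set, the view blends to it while player movement is disabled, then returns and restores walking.
; Tick steps a Lerp alpha per frame and offsets from the current Z, so motion accelerates, depends on frame rate and accumulates well beyond MoveDoorAmount.
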(event Custom|KeyCollected
  (bind _camera (Variables|Default|GetCamera))
  (Math|Integer|IncrementInt (Variables|Default|GetCollectedAmount)
    (:%20%20
      (if (== (Variables|Default|GetKeysRequired) (Variables|Default|GetCollectedAmount))
        (if (Utilities|IsValid _camera)
          (Game|Player|SetViewTargetwithBlend (Game|GetPlayerController 0) _camera 1.5 "VTBlend_Linear" 0.5 false)
          (Utilities|FlowControl|Delay 1.0)
          (Variables|Default|SetOpening true)
          (bind _asbp_player_character (Utilities|Casting|CastToBP_PlayerCharacter (Game|GetPlayerCharacter 0)))
          (Pawn|Components|CharacterMovement|DisableMovement (Variables|/Script/Engine.Character|GetCharacterMovement _asbp_player_character))
          (Utilities|FlowControl|Delay 2.0)
          (Game|Player|SetViewTargetwithBlend (Game|GetPlayerController 0) _asbp_player_character 2.0 "VTBlend_Linear" 0.5 false)
          (Pawn|Components|CharacterMovement|SetMovementMode (Variables|/Script/Engine.Character|GetCharacterMovement _asbp_player_character) "MOVE_Walking" 0)
          (else
            (Variables|Default|SetOpening true)))))))

(event EventBeginPlay)

(event Collision|EventActorBeginOverlap
  (params (OtherActor :type Actor%20Object%20Reference)))

(event EventTick
  (params (DeltaSeconds :type Float%20%28single-precision%29))
  (bind _defaultsceneroot (Variables|Default|GetDefaultSceneRoot))
  (bind _returnvalue (Transformation|GetWorldLocation _defaultsceneroot))
  (if (and (Variables|Default|GetOpening) (< (Variables|Default|Getlerp) 1.0))
    (Variables|Default|Setlerp (+ (Variables|Default|Getlerp) 0.01))
    (Transformation|SetWorldLocation _defaultsceneroot (Math|Vector|MakeVector (.x _returnvalue) (.y _returnvalue) (Math|Float|Lerp (.z _returnvalue) (+ (.z _returnvalue) (Variables|Default|GetMove%20door%20amount)) (Variables|Default|Getlerp))) false false)
    (if (> (Variables|Default|Getlerp) 1.0)
      (Variables|Default|SetOpening false))))

(fn ConstructionScript)