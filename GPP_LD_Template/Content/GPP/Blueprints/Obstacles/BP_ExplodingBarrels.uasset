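; BP_ExplodingBarrels is an obstacle that lights a fuse when its mesh is first hit and explodes when the timer runs out.
; The hit attaches a Niagara fuse effect, and Tick counts down before calling the explodable component and destroying the actor.
; The freezable component receives a dynamic material instance at BeginPlay and, while frozen, halts the countdown and pauses the fuse effect.
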(event OnComponentHit(StaticMesh)
  (params (HitComponent :type Primitive%20Component%20Object%20Reference) (OtherActor :type Actor%20Object%20Reference) (OtherComp :type Primitive%20Component%20Object%20Reference) (NormalImpulse :type Vector :default "0, 0, 0") (Hit :type Hit%20Result%20Structure%20%28by%20ref%29))
  ;[0.4491 0.8591 1] Handle collision hit
  ;;[0.4491 0.8591 1] Spawn Fuse PS
  (if (== (Variables|Default|GetFusePS) 0)
    (bind _returnvalue (Niagara|SpawnSystemAttached "/Game/GPP/Particles/NS_Fuse.NS_Fuse" (Variables|Default|GetStaticMesh) "" "0, 0, 0" "0, 0, 0" "SnapToTarget" false))
    (Variables|Default|SetFusePS _returnvalue)
    ;;[0.4491 0.8591 1] Start timer
    (Variables|Default|SetFuseTimer (Variables|Default|GetFuseTime))
    (Variables|Default|SetIsTriggered true)))

(event Custom|OnFrozenChanged
  (params (IsFrozen :type Boolean))
  ;[0.4491 0.8591 1] Initialise
  ;;[0.4491 0.8591 1] Bind to the on freoze changed event
  (if IsFrozen
    (bind _fuseps (Variables|Default|GetFusePS)
      (:then
        (Class|NiagaraComponent|SetPaused _fuseps true))
      (:else))
    (else
      (bind _fuseps_2 (Variables|Default|GetFusePS)
        (:then
          (Class|NiagaraComponent|SetPaused _fuseps_2 false))
        (:else)))))

(event EventBeginPlay
  (bind _bp_freezablecomponent (Variables|Default|GetBP_FreezableComponent))
  (bind _staticmesh (Variables|Default|GetStaticMesh))
  ;[0.4491 0.8591 1] Initialise
  ;;[0.4491 0.8591 1] Initialise the freeze component
  (bind _returnvalue (Rendering|Material|CreateDynamicMaterialInstance (Rendering|Material|GetMaterial _staticmesh 0) "None" "None" :!class /Script/Engine.KismetMaterialLibrary))
  (Rendering|Material|SetMaterial _staticmesh 0 _returnvalue)
  (Default|InitMaterial _bp_freezablecomponent (Utilities|Array|MakeArray _returnvalue))
  (Default|InitFreezeStatus _bp_freezablecomponent)
  ;;[0.4491 0.8591 1] Bind to the on freoze changed event
  (EventDispatchers|BindEventtoOnFrozenChanged _bp_freezablecomponent (delegate Custom|OnFrozenChanged)))

(event EventTick
  (params (DeltaSeconds :type Float%20%28single-precision%29))
  ;[0.4491 0.8591 1] Tick
  ;;[0.4491 0.8591 1] Check if timer can tick down
  (if (and (Variables|Default|GetIsTriggered) (not (Default|GetIsFrozen (Variables|Default|GetBP_FreezableComponent))))
    ;;[0.4491 0.8591 1] Count down fuse timer
    (bind _output_get (Variables|Default|SetFuseTimer (- (Variables|Default|GetFuseTimer) DeltaSeconds)))
    (if (< _output_get 0.0)
      ;;[0.4491 0.8591 1] Explode
      (Default|Explode (Variables|Default|GetBP_ExplodableComponent))
      (Actor|DestroyActor))))

(event EventDestroyed
  ;[0.4491 0.8591 1] Initialise
  ;;[0.4491 0.8591 1] Bind to the on freoze changed event
  (EventDispatchers|UnbindEventfromOnFrozenChanged (Variables|Default|GetBP_FreezableComponent) (delegate Custom|OnFrozenChanged)))

(fn ConstructionScript)