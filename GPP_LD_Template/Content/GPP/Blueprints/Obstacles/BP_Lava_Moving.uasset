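; BP_Lava_Moving is a lava obstacle that shuttles its mesh endlessly back and forth between a start point and an end point.
; BeginPlay calls the parent, snaps the mesh to the start and begins moving after a delay.
; A Timeline, with play rate set by MoveSpeed, lerps the mesh between the points' world locations.
; When it finishes, the endpoints swap and movement repeats after the same delay.
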(event Custom|MoveToTarget
  ;[0.4491 0.8591 1] Move to target points
  (bind _alpha (Timeline|Timeline PlayFromStart)
    (:Update
      ;;[0.4491 0.8591 1] Lerp between points
      (Transformation|SetWorldLocation (Variables|Character|GetMesh) (Math|Vector|Lerp(Vector) (Transformation|GetWorldLocation (Variables|Default|GetCurrentPoint)) (Transformation|GetWorldLocation (Variables|Default|GetTargetPoint)) _alpha) false false))
    (:Finished
      (Variables|Default|SetIs%20Heading%20To%20End%20Point (not (Variables|Default|GetIs%20Heading%20To%20End%20Point)))
      ;;[0.4491 0.8591 1] Flip targets
      (Variables|Default|SetTempPoint (Variables|Default|GetTargetPoint))
      (Variables|Default|SetTargetPoint (Variables|Default|GetCurrentPoint))
      (Variables|Default|SetCurrentPoint (Variables|Default|GetTempPoint))
      (Utilities|FlowControl|Delay (Variables|Default|GetDelay%20Between%20Points))
      (CallFunction|MovetoTarget))))

(event EventBeginPlay
  ;[0.4491 0.8591 1] Init
  ;;[0.4491 0.8591 1] Initialise to the start location
  (|CallParentFunction)
  (Transformation|SetWorldLocation (Variables|Character|GetMesh) (Transformation|GetWorldLocation (Variables|Default|GetStartPoint)) false true)
  ;;[0.4491 0.8591 1] Set target and current points
  (Variables|Default|SetTargetPoint (Variables|Default|GetEndPoint))
  (Variables|Default|SetIs%20Heading%20To%20End%20Point true)
  (Variables|Default|SetCurrentPoint (Variables|Default|GetStartPoint))
  (Utilities|FlowControl|Delay (Variables|Default|GetDelay%20Between%20Points))
  (CallFunction|MovetoTarget)
  (Components|Timeline|SetPlayRate (Variables|Default|GetTimeline) (Variables|Default|GetMoveSpeed)))

(event Collision|EventActorBeginOverlap
  (params (OtherActor :type Actor%20Object%20Reference)))

(event EventTick
  (params (DeltaSeconds :type Float%20%28single-precision%29)))

(fn ConstructionScript
  (|CallParentFunction))